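; BP_Trim is an actor with two point lights that can blink.
; While ShouldBlink is true, Tick sets both lights' intensity from the same scaled sine of game time, so they pulse in sync.
; The sine is not remapped, so the intensity value goes negative for half of each cycle.
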(event `self.ReceiveTick`
  (params (DeltaSeconds :type "Float (single-precision)"))
  (bind _returnvalue (* (`KismetMathLibrary.Sin` (* (`GameplayStatics.GetTimeSeconds`) (* 360.0 0.015))) 30000.0))
  (if (`self.ShouldBlink`)
    (`LightComponent.SetIntensity` (`self.PointLight`) _returnvalue)
    (`LightComponent.SetIntensity` (`self.PointLight1`) _returnvalue)))

(fn `UserConstructionScript`)